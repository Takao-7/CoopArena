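; Master Blueprint for DENT destructibles that breaks its destructible component when a kill switch event fires.
; The DENT_KillSwitch event calls DentKillSwitchFunction, which applies damage and impulse at the component's world location using switch-specific variables.
; The impulse direction is that world location doubled, so it depends on placement in the level rather than a chosen vector.
; BeginPlay and the construction script only call their parents.
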(event Custom|DENT_KillSwitch
  ;[0.07451 0.1216 0.2706] Kill Switch called
  (CallFunction|DentKillSwitchFunction))

(event EventBeginPlay
  (|CallParentFunction))

(event Collision|EventActorBeginOverlap
  (params (OtherActor :type Actor%20Object%20Reference)))

(event EventTick
  (params (DeltaSeconds :type Float%20%28single-precision%29)))

(fn ConstructionScript
  (|CallParentFunction))

(fn DentKillSwitchFunction
  (bind _destructible (Variables|Default|GetDestructible))
  (bind _returnvalue (Transformation|GetWorldLocation _destructible))
  ;[0.2706 0.2706 0.2706] Process Container
  ;;[0.07451 0.1216 0.2706] Get Location of DM and apply Damage
  (Game|Damage|ApplyDamage _destructible (Variables|DENT|KillSwitch|GetDamageOnSwitch) _returnvalue (* _returnvalue 2.0) (Variables|DENT|KillSwitch|GetImpulseOnSwitch)))