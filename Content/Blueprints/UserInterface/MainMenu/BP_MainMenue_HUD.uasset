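; Main menu HUD Blueprint whose only active logic restores game-only input mode on the first player controller when it is destroyed.
; BeginPlay is empty, and the chain that would create the WP_MainMenu widget, show the cursor, set UI-only input and add the widget to the viewport is disconnected.
; As it stands, this Blueprint never displays the menu itself.
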(event EventBeginPlay)

(event EventDestroyed
  (Input|SetInputModeGameOnly (Game|GetPlayerController 0)))

(fn ConstructionScript)