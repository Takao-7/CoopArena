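; Default in-game HUD Blueprint on a C++ base, showing ammo and fire-mode status, wave messages and the game-over screen.
; On Tick, rather than BeginPlay, it waits for a possessed player character, creates and initializes the widgets, then disables ticking.
; Fire, reload and fire-mode handlers update the ammo widget.
; SetState shows it while playing; spectating or match end hides it and opens the game-over screen with UI-only input.
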(event EventTick
  (params (DeltaSeconds :type Float%20%28single-precision%29))
  ;[0.2416 0 0.5866] Tick. We use the tick function here, because when BeginPlay is called, we might not have a owning pawn!
  (Utilities|IsValid (Game|Player|GetOwningPlayerController)
    (:Is%20Valid
      (bind _asplayer_character (Utilities|Casting|CastToPlayerCharacter (Class|HUD|GetOwningPawn)))
      (Utilities|FlowControl|Sequence
        (:then_0
          (CallFunction|CreateAmmoWidget)
          (bind _returnvalue (UserInterface|CreateWidget "/Game/Blueprints/UserInterface/Ingame/WBP_WaveMessage.WBP_WaveMessage_C"))
          (UserInterface|Viewport|AddtoViewport _returnvalue 0))
        (:then_1
          (Class|DefaultHUD|Init _asplayer_character)
          (Utilities|SetSmmoStatusValues))
        (:then_2
          (Actor|Tick|SetActorTickEnabled false))))))

(event EventHandleonReloadingFinishedK2
  (params (NumMagazines :type Integer) (NumRoundsInMagazine :type Integer))
  (bind _ammo_status (Variables|Default|GetAmmo%20status))
  ;[0.3478 0.4735 0] Handle ammo status changes
  (Default|SetNumberOfMagazinesLeft _ammo_status NumMagazines)
  (Default|SetNumberOfRoundsLeft _ammo_status NumRoundsInMagazine))

(event EventHandleonWeaponFireK2
  (params (NumRoundsLeft :type Integer))
  ;[0.3478 0.4735 0] Handle ammo status changes
  (Default|SetNumberOfRoundsLeft (Variables|Default|GetAmmo%20status) NumRoundsLeft))

(event EventSetState
  (params (State :type EHUDState%20Enum :default "MainMenu"))
  (bind _returnvalue (Game|Player|GetOwningPlayerController))
  (bind _ammo_status (Variables|Default|GetAmmo%20status))
  ;[0 0.5508 0.2705] Handle HUD state change
  (switch Utilities|FlowControl|Switch|SwitchonEHUDState State
    (:Playing
      (Widget|SetVisibility _ammo_status "Visible"))
    (:Spectating
      (Widget|SetVisibility _ammo_status "Hidden" :!label _label)
      (bind _returnvalue_2 (UserInterface|CreateWidget "/Game/Blueprints/UserInterface/Ingame/WBP_GameOverScreen.WBP_GameOverScreen_C" _returnvalue))
      (UserInterface|Viewport|AddtoViewport _returnvalue_2 0)
      (Input|SetInputModeUIOnly _returnvalue _returnvalue_2 "DoNotLock"))
    (:MatchEnd
      (goto _label))))

(event EventHandleonFireModeChangedK2
  (params (Character :type Humanoid%20Object%20Reference) (NewFireMode :type EFireMode%20Enum :default "Single"))
  ;[0.5701 0 0.2542] Handle fire mode changed
  (Default|SetFireMode (Variables|Default|GetAmmo%20status) NewFireMode))

(fn ConstructionScript)

(fn CreateAmmoWidget
  (bind _returnvalue (UserInterface|CreateWidget "/Game/Blueprints/UserInterface/Ingame/WBP_AmmoAndFireModeStatus.WBP_AmmoAndFireModeStatus_C" (Game|Player|GetOwningPlayerController)))
  (bind _output_get (Variables|Default|SetAmmo%20status _returnvalue))
  (Variables|Default|Set_AmmoStatusWidget _output_get) ; This is a variable from C++ and is used there to hide / display it
  (UserInterface|Viewport|AddtoViewport _output_get 0))