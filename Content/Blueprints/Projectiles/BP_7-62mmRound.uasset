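; BP_7-62mmRound is a 7.62mm bullet projectile Blueprint that can draw its flight path for debugging.
; It stores its location on BeginPlay, then each Tick, when DrawDebugFlyPath is set, draws a timed red line from the last stored location to the current one and updates that location.
; The construction script only calls the parent's, and the graphs here contain no movement or damage logic.
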(event EventTick
  (params (DeltaSeconds :type Float%20%28single-precision%29))
  (bind _returnvalue (Transformation|GetActorLocation))
  (if (Variables|Default|GetDraw%20debug%20fly%20path)
    (Rendering|Debug|DrawDebugLine (Variables|Default|GetLocation%20last%20frame) _returnvalue "(R=1.000000,G=0.039766,B=0.000000,A=1.000000)" 1e+01 0.0)
    (Variables|Default|SetLocation%20last%20frame _returnvalue)))

(event EventBeginPlay
  (Variables|Default|SetLocation%20last%20frame (Transformation|GetActorLocation)))

(fn ConstructionScript
  (|CallParentFunction))