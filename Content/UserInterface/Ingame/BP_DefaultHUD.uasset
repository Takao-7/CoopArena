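; BP_DefaultHUD is the in-game HUD that shows the player's ammo and fire mode status.
; On BeginPlay it initializes with the owning PlayerCharacter, then creates WBP_AmmoAndFireModeStatus and adds it to the viewport.
; K2 handlers for weapon fire, finished reloads and fire mode changes push round, magazine and mode updates into that widget.
; SetState shows the widget while Playing and hides it when Spectating or at Match End.
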(event EventBeginPlay
  ;[1 1 1] Begin Play
  (bind _asplayer_character (Utilities|Casting|CastToPlayerCharacter (Class|HUD|GetOwningPawn)))
  (Class|DefaultHUD|Init _asplayer_character)
  (bind _returnvalue (UserInterface|CreateWidget "/Game/UserInterface/Ingame/WBP_AmmoAndFireModeStatus.WBP_AmmoAndFireModeStatus_C" (Game|Player|GetOwningPlayerController)))
  (bind _output_get (Variables|Default|SetAmmo%20status _returnvalue))
  (Variables|Default|Set_AmmoStatusWidget _output_get)
  (UserInterface|Viewport|AddtoViewport _output_get 0))

(event EventSetState
  (params (State :type EHUDState%20Enum :default "Playing"))
  (bind _ammo_status (Variables|Default|GetAmmo%20status))
  ;[1 1 1] Handle HUD state change
  (switch Utilities|FlowControl|Switch|SwitchonEHUDState State
    (:Playing
      (Widget|SetVisibility _ammo_status "Visible"))
    (:Spectating
      (Widget|SetVisibility _ammo_status "Hidden" :!label _label))
    (:MatchEnd
      (goto _label))))

(event EventHandleonFireModeChangedK2
  (params (Character :type Humanoid%20Object%20Reference) (NewFireMode :type EFireMode%20Enum :default "Single"))
  ;[1 1 1] Handle fire mode changed
  (Default|SetFireMode (Variables|Default|GetAmmo%20status) NewFireMode))

(event EventHandleonReloadingFinishedK2
  (params (NumMagazines :type Integer) (NumRoundsInMagazine :type Integer))
  (bind _ammo_status (Variables|Default|GetAmmo%20status))
  ;[1 1 1] Handle ammo status changes
  (Default|SetNumberOfMagazinesLeft _ammo_status NumMagazines)
  (Default|SetNumberOfRoundsLeft _ammo_status NumRoundsInMagazine))

(event EventHandleonWeaponFireK2
  (params (NumRoundsLeft :type Integer))
  ;[1 1 1] Handle ammo status changes
  (Default|SetNumberOfRoundsLeft (Variables|Default|GetAmmo%20status) NumRoundsLeft))

(fn ConstructionScript)