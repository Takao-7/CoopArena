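; BP_Test is a test Blueprint for rotating one arrow component to match another.
; On BeginPlay it copies Arrow's world rotation directly onto Arrow2.
; Two disconnected experiments derive the rotation from cross-product axis and dot-product angle: one using forward vectors, marked working, the other normalized world locations, marked not working.
; The construction script and OnBeginLineTraceOver are empty.
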(event EventBeginPlay
  (Transformation|SetWorldRotation (Variables|Default|GetArrow2) (Transformation|GetWorldRotation (Variables|Default|GetArrow)) false false))

(fn ConstructionScript)

(fn OnBeginLineTraceOver
  (params (Pawn :type Pawn%20Object%20Reference))
  (return 0))