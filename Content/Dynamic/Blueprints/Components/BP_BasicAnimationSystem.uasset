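; Actor component that derives locomotion and aim state for the owning character, apparently to drive its animation.
; Each tick it computes input direction, speed, aim yaw/pitch and turn-on-spot state, then applies crouch/sprint overrides and reads weapon type through BP_BASInterface.
; Near-180° input reversals flip forward/backward movement instead of turning around.
; Actor-rotation logic exists but is inactive: turn-to-movement is never called and controller-desired-rotation code is disconnected.
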(event EventBeginPlay
  ;[1 1 1] Begin Play
  (Variables|Default|SetCharacter%20Movement%20Component (Actor|GetComponentbyClass (Components|GetOwner) "/Script/Engine.CharacterMovementComponent"))
  (bind _asbp_basinterface (Utilities|Casting|CastToBP_BASInterface (Components|GetOwner)))
  (Variables|BasicAnimationSystem|SetBAS%20Interface _asbp_basinterface))

(event EventTick
  (params (DeltaSeconds :type Float%20%28single-precision%29))
  ;[1 1 1] Tick
  (Utilities|FlowControl|Sequence
    (:then_0
      (Utilities|SetInputDirection))
    (:then_1
      (Utilities|SetHorizontalSpeed))
    (:then_2
      (Utilities|SetAimYaw))
    (:then_3
      (Utilities|SetAimPitch))
    (:then_4
      (Utilities|TurnonSpot))
    (:then_5
      (Utilities|SetUseControllerDesiredRotation))
    (:then_6
      (Utilities|SetIsCrouching/Sprinting))
    (:then_7
      (Utilities|SetEquippedWeaponType))))

(fn VectorAngle
  (params (A :type Vector) (B :type Vector))
  (bind _returnvalue (Math|Vector|VectorLength B))
  (bind _returnvalue_2 (Math|Vector|VectorLength A))
  (bind _returnvalue_3 (* _returnvalue_2 _returnvalue))
  (return (select (== _returnvalue_3 0.0) 0.0 (Class|KismetMathLibrary|DegAcos (/ (Math|Vector|DotProduct A B) _returnvalue_3)))))

(fn GetMovementInputVectorLocalSpace
  (bind _returnvalue (Components|GetOwner))
  (return (Math|Transform|InverseTransformDirection (Math|Transform|MakeTransform (Transformation|GetActorLocation _returnvalue) (Variables|BasicAnimationSystem|GetBAS%20Control%20Rotation)) (Class|Pawn|GetLastMovementInputVector (Variables|/Script/Engine.Actor|GetInstigator _returnvalue)))))