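; Actor component for a basic animation system that derives a character's locomotion and aim state each tick.
; It computes speed, aim yaw and pitch, and input direction relative to control rotation, choosing idle, forward or backward movement with memory of the previous direction.
; Idle aim yaw beyond a threshold sets a turn-on-spot state, while controller-desired rotation is enabled only during movement.
; A manual turn-to-movement routine exists but is unused.
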(event EventBeginPlay
  (Variables|Default|SetCharacter%20Movement%20Component (Actor|GetComponentbyClass (Components|GetOwner) "/Script/Engine.CharacterMovementComponent")))

(event EventTick
  (params (DeltaSeconds :type Float%20%28single-precision%29))
  (bind _character_movement_component (Variables|Default|GetCharacter%20Movement%20Component))
  (Utilities|FlowControl|Sequence
    (:then_0
      (Utilities|SetInputDirection))
    (:then_1
      (Utilities|SetHorizontalSpeed))
    (:then_2
      (Utilities|SetAimYaw))
    (:then_3
      (Utilities|SetAimPitch))
    (:then_4
      (Utilities|TurnonSpot))
    (:then_5
      (if (Utilities|Enum|Equal(Enum) (Variables|BasicAnimationSystem|GetBAS%20Movement%20State) "NewEnumerator0")
        (Variables|/Script/Engine.CharacterMovementComponent|SetbUseControllerDesiredRotation _character_movement_component false)
        (else
          (Variables|/Script/Engine.CharacterMovementComponent|SetbUseControllerDesiredRotation _character_movement_component true))))))

(fn VectorAngle
  (params (A :type Vector) (B :type Vector))
  (bind _returnvalue (Math|Vector|VectorLength B))
  (bind _returnvalue_2 (Math|Vector|VectorLength A))
  (bind _returnvalue_3 (* _returnvalue_2 _returnvalue))
  (return (select (== _returnvalue_3 0.0) 0.0 (Class|KismetMathLibrary|DegAcos (/ (Math|Vector|DotProduct A B) _returnvalue_3)))))

(fn GetMovementInputVectorLocalSpace
  (bind _returnvalue (Components|GetOwner))
  (return (Math|Transform|InverseTransformDirection (Math|Transform|MakeTransform (Transformation|GetActorLocation _returnvalue) (Variables|BasicAnimationSystem|GetBAS%20Control%20Rotation)) (Class|Pawn|GetLastMovementInputVector (Variables|/Script/Engine.Actor|GetInstigator _returnvalue)))))