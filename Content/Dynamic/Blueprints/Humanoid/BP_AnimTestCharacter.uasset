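; BP_AnimTestCharacter is a humanoid test character for trying out animation through its BasicAnimationSystem.
; Each tick, it rotates an InputDirection component by the animation system's input direction and a ControlDirection component by control yaw relative to the actor, visualizing both.
; The third-person camera activates at BeginPlay, and the ChangeCamera action toggles both it and the first-person camera.
; Releasing Q calls PlayMontage on the mesh.
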(event EventBeginPlay
  (Components|Activation|Activate (Variables|Default|Get_ThirdPersonCamera) false))

(event EventTick
  (params (DeltaSeconds :type Float%20%28single-precision%29))
  (Transformation|SetRelativeRotation (Variables|Default|GetInput%20direction) (Math|Rotator|MakeRotator 0.0 0.0 (.InputDirection (Utilities|Struct|BreakBASVariables (Class|BasicAnimationSystemComponent|GetActorVariables (Variables|Default|GetBasicAnimationSystem))))) false false)
  (Transformation|SetRelativeRotation (Variables|Default|GetControl%20direction) (Math|Rotator|MakeRotator 0.0 0.0 (.yaw (Math|Transform|InverseTransformRotation (Transformation|GetActorTransform) (Pawn|GetControlRotation :!class /Script/Engine.Pawn)))) false false))

(event Input|ActionEvents|InputActionChangeCamera
  (params (Key :type Key%20Structure))
  (:Pressed
    (Components|Activation|ToggleActive (Variables|Default|Get_FirstPersonCamera))))

(event Input|KeyboardEvents|Q
  (params (Key :type Key%20Structure))
  (:Released
    (Animation|Montage|PlayMontage (Variables|Character|GetMesh) 0)))

(fn ConstructionScript)