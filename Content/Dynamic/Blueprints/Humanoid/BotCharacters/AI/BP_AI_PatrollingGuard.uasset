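; AI controller for a patrolling guard that tracks the player through sight and hearing.
; On possess, it sets up the BB_Patrol blackboard and runs the GuardBehaviour behavior tree.
; Perception updates from Player-tagged actors feed the blackboard: sight sets or clears Enemy and records LastSeenLocation, while hearing only updates that location.
; A debug helper prints the sensed actor and sense type but is not called here.
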(event OnTargetPerceptionUpdated(AIPerception)
  (params (Actor :type Actor%20Object%20Reference) (Stimulus :type AI%20Stimulus%20Structure))
  ;[1 1 1] On Target Perception Update (Enemy sensed)
  (CallFunction|UpdateBlackboard Stimulus Actor))

(event EventOnPossess
  (params (PossessedPawn :type Pawn%20Object%20Reference))
  ;[1 1 1] Event BeginPlay
  (Utilities|FlowControl|Sequence
    (:then_0
      (bind _blackboardcomponent (Class|AIController|UseBlackboard "/Game/Dynamic/Blueprints/Humanoid/BotCharacters/AI/BB_Patrol.BB_Patrol"))
      (AI|RunBehaviorTree "/Game/Dynamic/Blueprints/Humanoid/BotCharacters/AI/GuardBehaviour.GuardBehaviour")
      (Variables|Default|SetBlackboard%20Component _blackboardcomponent))
    (:then_1
      (Utilities|Casting|CastTo PossessedPawn)
      (Utilities|IsValid 0
        (:Is%20Valid
          (Variables|Default|Setself%20AHumannoid 0 0))
        (:Is%20Not%20Valid
          (Development|PrintText "AIController: Controlled Pawn is not valid!"))))))

(fn ConstructionScript)

(fn DebugPrintSensedActor
  (params (Object :type Object%20Object%20Reference) (Stimulus :type AI%20Stimulus%20Structure%20%28by%20ref%29))
  (bind _returnvalue (Class|AIPerceptionSystem|GetSenseClassforStimulus Stimulus))
  (Development|PrintString (Utilities|String|Append "Guard " (Utilities|GetObjectName (Pawn|GetControlledPawn)) " " (Utilities|GetClassDisplayName _returnvalue) " " (Utilities|GetDisplayName Object))))

(fn UpdateBlackboard
  (params (AI%20stimulus :type AI%20Stimulus%20Structure%20%28by%20ref%29) (Sensed%20actor :type Actor%20Object%20Reference))
  (bind (_age _expirationage _strength _stimuluslocation _receiverlocation _tag _bsuccessfullysensed) (Utilities|Struct|BreakAIStimulus AI%20stimulus))
  (bind _blackboard_component (Variables|Default|GetBlackboard%20Component))
  (bind _lastseenlocation (Variables|Default|GetLastSeenLocation))
  (if (Actor|ActorHasTag Sensed%20actor "Player")
    (LocalVariables|SetSensed_Actor Sensed%20actor)
    (bind _returnvalue (Class|AIPerceptionSystem|GetSenseClassforStimulus AI%20stimulus))
    (if (Utilities|Enum|Equal(Enum) (Utilities|GetClassDisplayName _returnvalue) (LocalVariables|GetSense%20Sight))
      (if _bsuccessfullysensed
        (AI|Components|Blackboard|SetValueasObject _blackboard_component (LocalVariables|GetEnemy) (LocalVariables|GetSensed_Actor))
        (AI|Components|Blackboard|SetValueasVector _blackboard_component (Variables|Default|GetLastSeenLocation) _stimuluslocation)
        (else
          (AI|Components|Blackboard|SetValueasVector _blackboard_component _lastseenlocation _stimuluslocation)
          (AI|Components|Blackboard|ClearValue _blackboard_component (LocalVariables|GetEnemy))))
      (elif (Utilities|Enum|Equal(Enum) (Utilities|GetClassDisplayName _returnvalue) (LocalVariables|GetSense%20Hearing))
        (AI|Components|Blackboard|SetValueasVector _blackboard_component _lastseenlocation _stimuluslocation)))))