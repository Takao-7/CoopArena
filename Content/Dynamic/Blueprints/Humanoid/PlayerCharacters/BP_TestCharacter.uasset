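; BP_TestCharacter is a test player character that visualizes movement and aim state and adds a temporary HUD on BeginPlay.
; Each Tick orients indicator components to control yaw, velocity direction and the aim yaw from BASComponent, holding the last velocity rotation while stationary.
; Text components display aim yaw and horizontal velocity read from BASComponent.
; The ChangeCamera input toggles the first- and third-person cameras.
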(event EventTick
  (params (DeltaSeconds :type Float%20%28single-precision%29))
  (bind _returnvalue (Transformation|GetVelocity))
  (bind _velocity (Variables|Default|GetVelocity))
  (bind _bascomponent (Variables|Default|GetBASComponent))
  (bind _returnvalue_2 (Class|BasicAnimationSystemComponent|GetActorVariables _bascomponent))
  (bind _returnvalue_3 (Math|Conversions|RotationFromXVector _returnvalue))
  (bind (_aimyaw _aimpitch _horizontalvelocity) (Utilities|Struct|BreakBASVariables _returnvalue_2))
  (Transformation|SetWorldRotation (Variables|Default|GetView%20direction) (Math|Rotator|MakeRotator 0.0 0.0 (.yaw (Pawn|GetControlRotation :!class /Script/Engine.Pawn))) false false)
  (if (Math|Float|NearlyEqual(Float) (Math|Vector|VectorLength (Transformation|GetVelocity)) 0.0 0.1)
    (Transformation|SetWorldRotation _velocity (Variables|Default|GetVelocity%20rotation) false false)
    (else
      (Transformation|SetWorldRotation _velocity _returnvalue_3 false false)
      (Variables|Default|SetVelocity%20rotation _returnvalue_3)))
  (Transformation|SetRelativeRotation (Variables|Default|GetAim%20Yaw) (Math|Rotator|MakeRotator 0.0 0.0 _aimyaw) false false)
  (Rendering|Components|TextRender|SetText (Variables|Default|GetAim%20yaw%20text) (Utilities|Text|ToText(String) (Utilities|String|Append "Aim yaw: " (Utilities|String|ToString(Integer) (Math|Float|Truncate _aimyaw)))))
  (Rendering|Components|TextRender|SetText (Variables|Default|GetVelocity%20text) (Utilities|Text|ToText(String) (Utilities|String|Append "Velocity: " (Utilities|String|ToString(Integer) (Math|Float|Truncate _horizontalvelocity))))))

(event EventBeginPlay
  (bind _returnvalue (Game|GetPlayerController 0))
  ;[1 1 1] Begin Play
  (Utilities|IsValid _returnvalue
    (:Is%20Valid
      (bind _returnvalue_2 (UserInterface|CreateWidget "/Game/Dynamic/UserInterface/WBP_TempHUD.WBP_TempHUD_C" _returnvalue))
      (Utilities|IsValid _returnvalue_2
        (:Is%20Valid
          (UserInterface|Viewport|AddtoViewport _returnvalue_2 0))))))

(event Input|ActionEvents|InputActionChangeCamera
  (params (Key :type Key%20Structure))
  ;[1 1 1] Change camera
  (:Pressed
    (Components|Activation|ToggleActive (Variables|Default|Get_FirstPersonCamera))))

(fn ConstructionScript)