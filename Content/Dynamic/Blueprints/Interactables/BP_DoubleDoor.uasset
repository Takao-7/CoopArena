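; BP_DoubleDoor is an interactable double door that pairs two Door child actors, Door1 and Door2.
; On BeginPlay it casts each child actor to Door and copies its own OpeningAngle and DoubleSidedOpening settings onto both.
; The second door receives the negated angle, so the two open as mirror images.
; The Blueprint only configures the doors and holds no opening logic of its own.
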(event EventBeginPlay
  (Utilities|FlowControl|Sequence
    (:then_0
      (bind _asdoor (Utilities|Casting|CastToDoor (Variables|/Script/Engine.ChildActorComponent|GetChildActor (Variables|Default|GetDoor1))))
      (Variables|/Script/CoopArena.Door|SetOpeningAngle _asdoor (Variables|Door|GetOpening%20Angle))
      (Variables|/Script/CoopArena.Door|SetbTwoSidedOpening _asdoor (Variables|Door|GetDouble%20sided%20opening?)))
    (:then_1
      (bind _asdoor_2 (Utilities|Casting|CastToDoor (Variables|/Script/Engine.ChildActorComponent|GetChildActor (Variables|Default|GetDoor2))))
      (Variables|/Script/CoopArena.Door|SetOpeningAngle _asdoor_2 (* (Variables|Door|GetOpening%20Angle) -1.0))
      (Variables|/Script/CoopArena.Door|SetbTwoSidedOpening _asdoor_2 (Variables|Door|GetDouble%20sided%20opening?)))))

(fn ConstructionScript)