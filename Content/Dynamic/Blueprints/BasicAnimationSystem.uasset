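; BasicAnimationSystem is a component that computes locomotion and aim state for its owning character, apparently for animation, and rotates it while moving.
; Each tick it derives input direction, horizontal speed, forward/backward movement and aim yaw/pitch from control rotation, velocity and last input.
; Moving actors interpolate toward input direction, flipped when moving backward.
; Idle actors only get a turn-on-spot state; sharp velocity-to-input angles print for debugging.
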(event EventTick
  (params (DeltaSeconds :type Float%20%28single-precision%29))
  (bind _returnvalue (Components|GetOwner))
  (bind _returnvalue_2 (Transformation|GetVelocity _returnvalue))
  (bind _instigator (Variables|/Script/Engine.Actor|GetInstigator _returnvalue))
  (bind _returnvalue_3 (Class|Pawn|GetLastMovementInputVector _instigator))
  (bind _angle (CallFunction|VectorAngle _returnvalue_2 _returnvalue_3))
  (Utilities|FlowControl|Sequence
    (:then_0
      (Utilities|SetInputDirection))
    (:then_1
      (Utilities|SetHorizontalSpeed))
    (:then_2
      (Utilities|SetIsMovingForward))
    (:then_3
      (Utilities|SetAimYaw))
    (:then_4
      (Utilities|SetAimPitch))
    (:then_5
      (Utilities|TurnonSpot))
    (:then_6
      (if (>= _angle 1.2e+02)
        (Development|PrintString (Utilities|String|ToString(Float) _angle))))
    (:then_7
      (Utilities|TurnActortoMovement))))

(fn VectorAngle
  (params (A :type Vector) (B :type Vector))
  (bind _returnvalue (Math|Vector|VectorLength B))
  (bind _returnvalue_2 (Math|Vector|VectorLength A))
  (bind _returnvalue_3 (* _returnvalue_2 _returnvalue))
  (return (select (== _returnvalue_3 0.0) 0.0 (Class|KismetMathLibrary|DegAcos (/ (Math|Vector|DotProduct A B) _returnvalue_3)))))