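; Plasma projectile actor that damages whatever it hits, then destroys itself.
; On hit, it ignores itself and calls ReceivePointDamage directly on targets that pass a cast, falling back to ApplyPointDamage for all others, crediting its instigator.
; It then spawns a short spark effect at the impact point, with an optional debug sphere marking the hit location.
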(event Collision|EventHit
  (params (MyComp :type Primitive%20Component%20Object%20Reference) (Other :type Actor%20Object%20Reference) (OtherComp :type Primitive%20Component%20Object%20Reference) (bSelfMoved :type Boolean) (HitLocation :type Vector :default "0, 0, 0") (HitNormal :type Vector :default "0, 0, 0") (NormalImpulse :type Vector :default "0, 0, 0") (Hit :type Hit%20Result%20Structure%20%28by%20ref%29))
  (bind _self self)
  (bind _damage (Variables|Default|GetDamage))
  (bind _returnvalue (Game|GetInstigatorController _self))
  (if (!= self Other) ; Check if we didn't hit ourself
    (bind _ashumannoid (Utilities|Casting|CastTo Other)
      (:then
        (CallFunction|ReceivePointDamage _ashumannoid _damage 0 HitLocation "0, 0, 0" 0 "None" HitNormal _returnvalue _self Hit))
      (:CastFailed
        (Game|Damage|ApplyPointDamage Other _damage HitNormal Hit _returnvalue _self)))
    (if (Variables|Default|GetbDebugHitLocation)
      (Rendering|Debug|DrawDebugSphere HitLocation 1e+01 12 "(R=1.000000,G=0.000000,B=0.062383,A=1.000000)" 2e+01))
    (Effects|SpawnEmitteratLocation "/Game/Static/StarterContent/Particles/P_SparksShort.P_SparksShort" (.ImpactPoint (Collision|BreakHitResult Hit)))
    (Actor|DestroyActor)))

(fn ConstructionScript)